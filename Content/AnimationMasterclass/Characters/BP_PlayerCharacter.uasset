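; Player character Blueprint that turns Enhanced Input into movement, stance and jump state variables.
; On possession by a player controller it adds the default mapping context and turns on the Enhanced Input debug display.
; Move events store the 2D input as a direction vector, crouch flips a standing flag, and jump sets a request flag.
; The graph only records these values and applies no movement itself.
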(event Input|EnhancedActionEvents|EnhancedInputActionIA_CrouchToggle
  (params (ActionValue :type Boolean) (ElapsedSeconds :type Float%20%28double-precision%29) (TriggeredSeconds :type Float%20%28double-precision%29) (InputAction :type Input%20Action%20Object%20Reference :default "/Game/Input/Actions/IA_CrouchToggle.IA_CrouchToggle"))
  (Variables|Animation|SetIsStanding (not (Variables|Animation|GetIsStanding))))

(event Input|EnhancedActionEvents|EnhancedInputActionIA_Move
  (params (ActionValue :type Vector%202D%20Structure) (ElapsedSeconds :type Float%20%28double-precision%29) (TriggeredSeconds :type Float%20%28double-precision%29) (InputAction :type Input%20Action%20Object%20Reference :default "/Game/Input/Actions/IA_Move.IA_Move"))
  (:Triggered
    (Variables|Animation|SetInputMovementDirection (Math|Vector|MakeVector (.x ActionValue) (.y ActionValue) 0.0) :!label _label))
  (:Started
    (goto _label))
  (:Canceled
    (goto _label))
  (:Completed
    (goto _label)))

(event Input|EnhancedActionEvents|EnhancedInputActionIA_Jump
  (params (ActionValue :type Boolean) (ElapsedSeconds :type Float%20%28double-precision%29) (TriggeredSeconds :type Float%20%28double-precision%29) (InputAction :type Input%20Action%20Object%20Reference :default "/Game/Input/Actions/IA_Jump.IA_Jump"))
  (:Triggered
    (Variables|Animation|SetRequestedJump true)))

(event EventPossessed
  (params (NewController :type Controller%20Object%20Reference))
  ;[0.15 0.15 0.15 0.5] When Possessing We Check If It's A Player And Add The Mappings According To The Actions We Want To Do.
  (bind _asplayer_controller (Utilities|Casting|CastToPlayerController NewController))
  (Input|AddMappingContext (PlayerController|LocalPlayerSubsystems|GetEnhancedInputLocalPlayerSubsystem _asplayer_controller) "/Game/Input/IMC_Default.IMC_Default" 0 "(bIgnoreAllPressedKeysUntilRelease=True,bForceImmediately=False,bNotifyUserSettings=False)") ; We Edited This IMC_Default To Add The Jump
  (Development|ExecuteConsoleCommand "showdebug enhancedinput" 0))

(fn ConstructionScript)