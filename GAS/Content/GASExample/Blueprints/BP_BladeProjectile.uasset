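; BP_BladeProjectile is a homing blade projectile for the Warpstrike ability.
; Each tick it makes a swept move toward its Target actor at ProjectileSpeed, facing along the freshly computed direction.
; When its static mesh hits any actor other than Parent, it sends the Warpstrike ArrivedAtPoint gameplay event to Parent and destroys itself.
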(event OnComponentHit(StaticMesh)
  (params (HitComponent :type Primitive%20Component%20Object%20Reference) (OtherActor :type Actor%20Object%20Reference) (OtherComp :type Primitive%20Component%20Object%20Reference) (NormalImpulse :type Vector :default "0, 0, 0") (Hit :type Hit%20Result%20Structure%20%28by%20ref%29))
  (if (not (== OtherActor (Variables|Default|GetParent)))
    (Ability|SendGameplayEventtoActor (Variables|Default|GetParent) "(TagName=\"Abilities.Warpstrike.ArrivedAtPoint\")")
    (Actor|DestroyActor)))

(event EventTick
  (params (DeltaSeconds :type Float%20%28single-precision%29))
  (Transformation|SetActorLocationAndRotation (+ (Transformation|GetActorLocation) (* (CallFunction|GetDirectiontoTarget) (* (Variables|Default|GetProjectileSpeed) DeltaSeconds))) (Math|Rotator|MakeRotfromX (CallFunction|GetDirectiontoTarget)) true))

(fn ConstructionScript)

(fn GetDirectiontoTarget
  (return (Math|Vector|GetUnitDirection(Vector) (Transformation|GetActorLocation) (Transformation|GetActorLocation (Variables|Default|GetTarget)))))