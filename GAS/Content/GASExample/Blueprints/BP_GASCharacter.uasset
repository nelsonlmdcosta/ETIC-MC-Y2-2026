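; Player character Blueprint for a Gameplay Ability System example, with warp strike, dash and sword equipping.
; BeginPlay activates the equip ability once, grants warp strike and dash, applies health and mana regen effects, and shows a stat viewer widget.
; Debug keys trigger both abilities, random damage and stackable poison.
; AnyDamage converts incoming damage into a GameplayEffect spec using a SetByCaller magnitude, keeping the amount dynamic.
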(event EventBeginPlay
  (bind _abilitysystemcomponent (Variables|Default|GetAbilitySystemComponent))
  (|CallParentFunction)
  (Utilities|FlowControl|Sequence
    (:then_0
      (bind _returnvalue (Class|AbilitySystemComponent|GiveAbilityandActivateOnce (Variables|Default|GetAbilitySystemComponent) "/Game/GASExample/GAS/Abilities/GA_EquipEngineSword.GA_EquipEngineSword_C" 0 -1)) ; Use an ability to equip the weapon and all the logic associated to it
      (Variables|Default|SetEquippedWeaponAbility _returnvalue)
      (GameplayAbilities|GiveAbility _abilitysystemcomponent "/Game/GASExample/GAS/Abilities/GA_FFXV_WarpStrike.GA_FFXV_WarpStrike_C" 0 -1) ; Warp Strike is an ability for the player independant fro the weapon so we equip it here
      (GameplayAbilities|GiveAbility _abilitysystemcomponent "/Game/GASExample/GAS/Abilities/GA_Dash.GA_Dash_C" 0 -1)
      (GameplayEffects|ApplyGameplayEffectToSelf :self (Variables|Default|GetAbilitySystemComponent) :GameplayEffectClass "/Game/GASExample/GAS/Effects/GE_HealthRegen.GE_HealthRegen_C")
      (GameplayEffects|ApplyGameplayEffectToSelf :self (Variables|Default|GetAbilitySystemComponent) :GameplayEffectClass "/Game/GASExample/GAS/Effects/GE_ManaRegen.GE_ManaRegen_C"))
    (:then_1
      (bind _returnvalue_2 (UserInterface|CreateWidget "/Game/GASExample/Widgets/WBP_StatViewer.WBP_StatViewer_C"))
      (UserInterface|Viewport|AddtoViewport _returnvalue_2 0))))

(event Game|Damage|EventAnyDamage
  (params (Damage :type Float%20%28single-precision%29) (DamageType :type Damage%20Type%20Object%20Reference) (InstigatedBy :type Controller%20Object%20Reference) (DamageCauser :type Actor%20Object%20Reference))
  (bind _returnvalue (Ability|GameplayEffect|AssignTagSetbyCallerMagnitude (GameplayEffects|MakeOutgoingSpec :self (Variables|Default|GetAbilitySystemComponent) :GameplayEffectClass "/Game/GASExample/GAS/Effects/GE_DealDamage.GE_DealDamage_C") "(TagName=\"Damage.Magnitude\")" Damage))
  (GameplayEffects|ApplyGameplayEffectSpecToSelf (Variables|Default|GetAbilitySystemComponent) _returnvalue) ; Completly dynamic
)

(event Input|KeyboardEvents|DebugKeyP
  (params (Key :type Key%20Structure :default "None") (ActionValue :type Input%20Action%20Value%20Structure))
  (:Pressed
    (GameplayEffects|ApplyGameplayEffectToSelf :self (Variables|Default|GetAbilitySystemComponent) :GameplayEffectClass "/Game/GASExample/GAS/Effects/GE_StackablePoison.GE_StackablePoison_C" :Level 0.0)))

(event Input|KeyboardEvents|DebugKeySubtract
  (params (Key :type Key%20Structure :default "None") (ActionValue :type Input%20Action%20Value%20Structure))
  (:Pressed
    (Game|Damage|ApplyDamage self (Math|Random|RandomFloatinRange -5.0 -25.0) 0 0 "/Script/Engine.DamageType")))

(event Input|KeyboardEvents|DebugKeyShiftLeftShift
  (params (Key :type Key%20Structure :default "None") (ActionValue :type Input%20Action%20Value%20Structure))
  (:Pressed
    (Abilities|TryActivateAbilitybyClass (Variables|Default|GetAbilitySystemComponent) "/Game/GASExample/GAS/Abilities/GA_Dash.GA_Dash_C" true)))

(event Input|MouseEvents|DebugKeyLeftMouseButton
  (params (Key :type Key%20Structure :default "None") (ActionValue :type Input%20Action%20Value%20Structure))
  (:Released
    (Abilities|TryActivateAbilitybyClass (Variables|Default|GetAbilitySystemComponent) "/Game/GASExample/GAS/Abilities/GA_FFXV_WarpStrike.GA_FFXV_WarpStrike_C" true)))

(fn ConstructionScript
  (|CallParentFunction))