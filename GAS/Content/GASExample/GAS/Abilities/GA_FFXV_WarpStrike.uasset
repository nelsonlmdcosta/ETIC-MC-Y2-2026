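; Gameplay ability for an FFXV-style warp strike that throws the avatar's blade at a target and teleports the avatar to it.
; On activation it commits, takes the first synchronous Targeting System result, turns to face it and plays a random slash montage.
; A throw gameplay event hides the mesh's first child component and spawns BP_BladeProjectile at the hand socket.
; An arrival event teleports the avatar to the projectile, restores visibility and ends the ability.
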(event Ability|EventActivateAbility
  (bind _returnvalue (Ability|GetAvatarActorfromActorInfo))
  (bind _returnvalue_2 (Ability|GetAvatarActorfromActorInfo))
  (bind _returnvalue_3 (Actor|GetComponentbyClass _returnvalue_2 "/Script/Engine.SkeletalMeshComponent"))
  (bind _returnvalue_4 (Components|GetChildComponent _returnvalue_3 0))
  (bind _returnvalue_5 (Ability|CommitAbility))
  (if _returnvalue_5
    (bind _targetinghandle (|PerformTargetingRequest (Ability|GetAvatarActorfromActorInfo) "/Game/GASExample/Targeting/DA_FFXV_TargetingPreset.DA_FFXV_TargetingPreset" false)
      (:Targeted
        (Utilities|IsValid (Utilities|Array|Get(acopy) (Class|TargetingSubsystem|GetTargetingResultsActors (GameInstanceSubsystems|GetTargetingSubsystem) _targetinghandle))
          (:Is%20Valid
            (bind _output_get (Variables|Default|SetTarget (Utilities|Array|Get(acopy) (Class|TargetingSubsystem|GetTargetingResultsActors (GameInstanceSubsystems|GetTargetingSubsystem) _targetinghandle))))
            (Utilities|FlowControl|Sequence
              (:then_0
                (Transformation|SetWorldRotation (Variables|/Script/Engine.Actor|GetRootComponent _returnvalue) (Math|Rotator|MakeRotator 0.0 0.0 (.yaw (Math|Rotator|FindLookatRotation (Transformation|GetActorLocation _returnvalue) (Transformation|GetActorLocation _output_get)))) false false))
              (:then_1
                (Animation|Montage|PlayMontage (Actor|GetComponentbyClass _returnvalue "/Script/Engine.SkeletalMeshComponent") (.OutItem (Utilities|Array|Random (Utilities|Array|MakeArray "/Game/GASExample/Animation/Sword_And_Shield_Slash_2_Montage.Sword_And_Shield_Slash_2_Montage" "/Game/GASExample/Animation/Sword_And_Shield_Slash_Montage.Sword_And_Shield_Slash_Montage")))
                  (:then
                    (Ability|Tasks|WaitGameplayEvent "(TagName=\"Abilities.Warpstrike.NotifyThrow\")" 0
                      (:EventReceived
                        (Rendering|SetVisibility _returnvalue_4 false false)
                        (bind _returnvalue_6 (Game|SpawnActorfromClass "/Game/GASExample/Blueprints/BP_BladeProjectile.BP_BladeProjectile_C" (Transformation|GetSocketTransform _returnvalue_3 "HandGrip_R" "RTS_World") "AlwaysSpawn" "MultiplyWithRoot" 0 (Ability|GetAvatarActorfromActorInfo) (Variables|Default|GetTarget) 0))
                        (Ability|Tasks|WaitGameplayEvent "(TagName=\"Abilities.Warpstrike.ArrivedAtPoint\")" 0
                          (:EventReceived
                            (Transformation|SetActorLocation (Ability|GetAvatarActorfromActorInfo) (Transformation|GetActorLocation _returnvalue_6) false true)
                            (Rendering|SetVisibility _returnvalue_4 true false)
                            (Ability|EndAbility))))))))))
          (:Is%20Not%20Valid
            (Ability|EndAbility)))))
    (else
      (Ability|EndAbility))))

(event Ability|EventOnEndAbility
  (params (bWasCancelled :type Boolean)))