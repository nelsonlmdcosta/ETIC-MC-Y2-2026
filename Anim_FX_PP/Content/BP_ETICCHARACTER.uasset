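; BP_ETICCHARACTER is a character Blueprint that shows on-screen debug readouts of its health changes.
; On BeginPlay it runs the parent logic, then binds to the HealthComponent's heal and damage events.
; Each handler prints the component's current normalized health, green for healing and red for damage, under a shared key so the latest message replaces the previous one.
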(event Custom|OnHealed
  (params (NormalizedHealth :type Float%20%28single-precision%29))
  (Development|PrintString (Utilities|String|ToString(Float) (Class|HealthComponent|GetNormalizedHealth (Variables|Default|GetHealthComponent))) true true "(R=0.030004,G=1.000000,B=0.000000,A=1.000000)" 2.0 "42069"))

(event Custom|Ondamaged
  (params (NormalizedHealth :type Float%20%28single-precision%29))
  (Development|PrintString (Utilities|String|ToString(Float) (Class|HealthComponent|GetNormalizedHealth (Variables|Default|GetHealthComponent))) true true "(R=1.000000,G=0.001898,B=0.000000,A=1.000000)" 2.0 "42069"))

(event EventBeginPlay
  (bind _healthcomponent (Variables|Default|GetHealthComponent))
  (|CallParentFunction)
  (EventDispatchers|BindEventtoOnDamageHealedEvent _healthcomponent (EventDispatchers|CreateEvent :!event Custom|OnHealed))
  (EventDispatchers|BindEventtoOnDamageReceivedEvent _healthcomponent (EventDispatchers|CreateEvent :!event Custom|Ondamaged)))

(fn ConstructionScript)